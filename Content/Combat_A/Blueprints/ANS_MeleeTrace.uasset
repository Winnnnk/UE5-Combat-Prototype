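; Anim notify state that drives the melee trace window on BP_PlayerCombatChar during animations.
; Begin calls the character's trace-begin function and tick calls its per-frame trace, so the hit logic lives on the character.
; Begin also prints a debug line with the animation, the character's current frame and the window width in frames at an assumed 60 fps.
; No end handler is present, and a duplicate begin branch is left unconnected.
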(fn ReceivedNotifyBegin
  (params (MeshComp :type Skeletal%20Mesh%20Component%20Object%20Reference) (Animation :type Anim%20Sequence%20Base%20Object%20Reference) (TotalDuration :type Float%20%28single-precision%29) (EventReference :type Anim%20Notify%20Event%20Reference%20Structure%20%28by%20ref%29))
  (bind _asbp_player_combat_char (Utilities|Casting|CastToBP_PlayerCombatChar (Components|GetOwner MeshComp))
    (:then
      (Default|FonTraceBegin _asbp_player_combat_char)
      (bind _frame (Default|FGetCurrentFrame _asbp_player_combat_char))
      (Development|PrintString _asbp_player_combat_char (Utilities|String|Append (Utilities|String|Append (Utilities|String|Append (Utilities|String|Append (Utilities|String|Append "TRACEWIN " (Utilities|String|ToString(Object) Animation)) "  start=") (Utilities|String|ToString(Integer) _frame)) "  width=") (Utilities|String|ToString(Float) (* TotalDuration (Math|Float|MakeLiteralFloat 6e+01)))) false true "(R=0.000000,G=0.660000,B=1.000000,A=1.000000)" 0.0)
      (return true))
    (:CastFailed
      (return false))))

(fn ReceivedNotifyTick
  (params (MeshComp :type Skeletal%20Mesh%20Component%20Object%20Reference) (Animation :type Anim%20Sequence%20Base%20Object%20Reference) (FrameDeltaTime :type Float%20%28single-precision%29) (EventReference :type Anim%20Notify%20Event%20Reference%20Structure%20%28by%20ref%29))
  (bind _asbp_player_combat_char (Utilities|Casting|CastToBP_PlayerCombatChar (Components|GetOwner MeshComp))
    (:then
      (Default|FTraceTick _asbp_player_combat_char)
      (return true))
    (:CastFailed
      (return false))))