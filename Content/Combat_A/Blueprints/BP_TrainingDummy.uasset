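; BP_TrainingDummy is a combat target that tracks health and poise and prints hit results as debug text.
; TakeCombatHit subtracts damage from health, clamped to its range, then reduces poise or zeroes it on a forced break.
; When positive poise is depleted, it refills to maximum and the function returns true to signal a break, otherwise false.
; The event graph holds only disabled stubs, and zero health triggers nothing.
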(event EventBeginPlay)

(event Collision|EventActorBeginOverlap
  (params (OtherActor :type Actor%20Object%20Reference)))

(event EventTick
  (params (DeltaSeconds :type Float%20%28single-precision%29)))

(fn ConstructionScript
  (|CallParentFunction))

(fn TakeCombatHit
  (params (Damage :type Float%20%28double-precision%29) (PoiseDamage :type Float%20%28double-precision%29) (bForceBreak :type Boolean) (Hit :type Hit%20Result%20Structure))
  (Variables|Default|SetHealth (Math|Float|Clamp(Float) (- (Variables|Default|GetHealth) Damage) 0.0 (Variables|Default|GetMaxHealth)))
  (if (> (Variables|Default|GetPoise) (Math|Float|MakeLiteralFloat 0.0))
    (if (<= (select bForceBreak (Math|Float|MakeLiteralFloat 0.0) (- (Variables|Default|GetPoise) PoiseDamage)) (Math|Float|MakeLiteralFloat 0.0))
      (Variables|Default|SetPoise (Variables|Default|GetMaxPoise))
      (Development|PrintString (Utilities|String|Append (Utilities|String|Append (Utilities|String|Append (Utilities|String|Append (Utilities|String|Append "[Dummy] POISE BREAK  hp " (Utilities|String|ToString(Float) (Variables|Default|GetHealth))) "/") (Utilities|String|ToString(Float) (Variables|Default|GetMaxHealth))) "  poise reset to ") (Utilities|String|ToString(Float) (Variables|Default|GetMaxPoise))) true true "(R=1.000000,G=0.550000,B=0.000000,A=1.000000)" 3.0)
      (return true)
      (else
        (Variables|Default|SetPoise (select bForceBreak (Math|Float|MakeLiteralFloat 0.0) (- (Variables|Default|GetPoise) PoiseDamage)))
        (Development|PrintString (Utilities|String|Append (Utilities|String|Append (Utilities|String|Append (Utilities|String|Append (Utilities|String|Append (Utilities|String|Append (Utilities|String|Append "[Dummy] hp " (Utilities|String|ToString(Float) (Variables|Default|GetHealth))) "/") (Utilities|String|ToString(Float) (Variables|Default|GetMaxHealth))) "  poise ") (Utilities|String|ToString(Float) (Variables|Default|GetPoise))) "/") (Utilities|String|ToString(Float) (Variables|Default|GetMaxPoise))) true true "(R=0.000000,G=0.660000,B=1.000000,A=1.000000)" 3.0)
        (return false)))
    (else
      (Variables|Default|SetPoise (Math|Float|Clamp(Float) (select bForceBreak (Math|Float|MakeLiteralFloat 0.0) (- (Variables|Default|GetPoise) PoiseDamage)) 0.0 (Variables|Default|GetMaxPoise)))
      (return false))))