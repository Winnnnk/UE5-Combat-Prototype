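; Boss enemy that turns to face the player and starts a montage attack from a data table row when in range and off cooldown.
; Montage position converted to 60 fps frames gates a bone sphere trace to the active window, sending one damage message per swing via I_Damageable.
; MeasureMode instead traces all swing long, logging contact frames.
; Per-actor slow motion uses CustomTimeDilation with a timed, lerped recovery; incoming hits just return false.
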(event EventBeginPlay
  (Variables|Default|SetTargetActor (Game|GetPlayerCharacter 0))
  (Development|PrintString "[Boss] BeginPlay ready" true true "(R=0.000000,G=0.660000,B=1.000000,A=1.000000)" 4.0))

(event Collision|EventActorBeginOverlap
  (params (OtherActor :type Actor%20Object%20Reference)))

(event EventTick
  (params (DeltaSeconds :type Float%20%28single-precision%29))
  (bind _returnvalue (Transformation|GetActorLocation))
  (bind _targetactor (Variables|Default|GetTargetActor))
  (bind _currentmovedata (Variables|Default|GetCurrentMoveData))
  (bind (_displayname _montage _sectionname _movecategory _startupframes _activestart _activeend) (Utilities|Struct|BreakS_AttackFrameData _currentmovedata))
  (bind _returnvalue_2 (Transformation|GetActorLocation _targetactor))
  (bind _returnvalue_3 (Math|Vector|Distance(Vector) _returnvalue _returnvalue_2))
  (CallFunction|FTickSlowMo)
  (bind _frame (CallFunction|FBossFrame))
  (if (Variables|Default|GetbAttacking)
    (if (< _frame (Class|KismetSystemLibrary|MakeLiteralInteger))
      (Variables|Default|SetbAttacking false)
      (Variables|Default|SetNextAttackReadyTime (+ (Utilities|Time|GetGameTimeinSeconds) (Variables|Default|GetAttackCooldownSec)))
      (Development|PrintString (Utilities|String|Append "[Boss] swing end dist=" (Utilities|String|ToString(Float) _returnvalue_3)) true true "(R=0.000000,G=0.660000,B=1.000000,A=1.000000)" 4.0)
      (elif (Variables|Default|GetbMeasureMode)
        (CallFunction|FBossTraceTick _frame)
        (elif (and (>= _frame _activestart) (<= _frame _activeend))
          (CallFunction|FBossTraceTick _frame))))
    (else
      (Utilities|IsValid _targetactor
        (:Is%20Valid
          (Transformation|SetActorRotation (Math|Rotator|MakeRotator 0.0 0.0 (.Yaw (Math|Rotator|BreakRotator (Math|Rotator|FindLookatRotation _returnvalue _returnvalue_2)))))
          (if (and (<= _returnvalue_3 (Variables|Default|GetAttackRangeCm)) (> (Utilities|Time|GetGameTimeinSeconds) (Variables|Default|GetNextAttackReadyTime)))
            (CallFunction|FBossStartAttack)))))))

(fn ConstructionScript)

(fn FBossFrame
  (bind _returnvalue (Animation|GetCurrentMontage :!class /Script/Engine.Character))
  (Utilities|IsValid _returnvalue
    (:Is%20Valid
      (return (Math|Float|Floor (* (Animation|Montage|MontageGetPosition (Components|SkeletalMesh|GetAnimInstance (Variables|Character|GetMesh)) _returnvalue) (Math|Float|MakeLiteralFloat 6e+01)))))
    (:Is%20Not%20Valid
      (return -1))))

(fn FBossStartAttack
  (bind _returnvalue (Utilities|GetDataTableRow (Variables|Default|GetDT_BossAttack) (Variables|Default|GetAttackMoveID))
    (:then
      (Variables|Default|SetCurrentMoveData _returnvalue)
      (bind _returnvalue_2 (Utilities|LoadAssetBlocking (.Montage (Utilities|Struct|BreakS_AttackFrameData _returnvalue))))
      (bind _as动画蒙太奇 (Utilities|Casting|CastToAnimMontage _returnvalue_2)
        (:then
          (Animation|PlayAnimMontage _as动画蒙太奇 1.0 "None")
          (Variables|Default|SetbAttacking true)
          (Variables|Default|SetbHitLandedThisSwing false)
          (Variables|Default|SetLastLoggedFrame -1)
          (Development|PrintString "[Boss] StartAttack"))
        (:CastFailed
          (Development|PrintString "[Boss] Montage 加载失败"))))
    (:RowNotFound
      (Development|PrintString "[Boss] 帧表找不到 AttackMoveID"))))

(fn FBossTraceTick
  (params (Frame :type Integer))
  (bind _mesh (Variables|Character|GetMesh))
  (bind _tracebonename (Variables|Default|GetTraceBoneName))
  (bind _currentmovedata (Variables|Default|GetCurrentMoveData))
  (bind (_displayname _montage _sectionname _movecategory _startupframes _activestart _activeend _totalframes _combocancelstart _nextcombomoveid _dodgecancelstart _iframestart _iframeend _motioncurve _motiondistance _motionframestart _motionframeend _damage _poisedamage _resolvegain _feedbacklevel _hitdeduppolicy _dedupintervalframes _bforcepoisebreak) (Utilities|Struct|BreakS_AttackFrameData _currentmovedata))
  (bind _returnvalue (Transformation|GetSocketLocation _mesh _tracebonename))
  (bind _outhits (Collision|MultiSphereTraceByChannel _returnvalue _returnvalue (Variables|Default|GetTraceRadius) "TraceTypeQuery1" false 0 "ForDuration" true "(R=1.000000,G=0.000000,B=0.000000,A=1.000000)" "(R=0.000000,G=1.000000,B=0.000000,A=1.000000)" 1.0))
  (for _array_element _outhits
    (if (Utilities|DoesObjectImplementInterface (.HitActor (Collision|BreakHitResult _array_element)) "/Game/Combat_A/Blueprints/I_Damageable.I_Damageable_C")
      (if (Variables|Default|GetbMeasureMode)
        (if (!= Frame (Variables|Default|GetLastLoggedFrame))
          (Variables|Default|SetLastLoggedFrame Frame)
          (Development|PrintString (Utilities|String|Append "[BossMeasure] contact frame=" (Utilities|String|ToString(Integer) Frame)) true true "(R=0.000000,G=0.660000,B=1.000000,A=1.000000)" 4.0))
        (elif (not (Variables|Default|GetbHitLandedThisSwing))
          (Variables|Default|SetbHitLandedThisSwing true)
          (Development|PrintString (Utilities|String|Append "[BossHit] frame=" (Utilities|String|ToString(Integer) Frame)) true true "(R=0.000000,G=0.660000,B=1.000000,A=1.000000)" 4.0)
          (Class|IDamageable|TakeCombatHit(Message) (.HitActor (Collision|BreakHitResult _array_element)) _damage _poisedamage _bforcepoisebreak _array_element))))))

(fn FExitSlowMo
  (Variables|Default|SetSlowMoRecoverFrom (Variables|Default|GetCustomTimeDilation))
  (Variables|Default|SetSlowMoRecoverStart (Utilities|Time|GetGameTimeinSeconds))
  (Variables|Default|SetbSlowMoRecovering true)
  (Development|PrintString "[SlowMo] exit ramp start" false true "(R=0.000000,G=0.660000,B=1.000000,A=1.000000)" 0.0))

(fn FEnterSlowMo
  (params (Scale :type Float%20%28double-precision%29) (RealSeconds :type Float%20%28double-precision%29))
  (Variables|Default|SetbSlowMoRecovering false)
  (Variables|Default|SetCustomTimeDilation Scale)
  (Utilities|Time|SetTimerbyFunctionName self "F_ExitSlowMo" RealSeconds)
  (Development|PrintString (Utilities|String|Append (Utilities|String|Append (Utilities|String|Append "[SlowMo] start scale=" (Utilities|String|ToString(Float) Scale)) " sec=") (Utilities|String|ToString(Float) RealSeconds)) false true "(R=0.000000,G=0.660000,B=1.000000,A=1.000000)" 0.0))

(fn FTickSlowMo
  (bind _returnvalue (Utilities|Time|GetGameTimeinSeconds))
  (bind _slowmorecoverstart (Variables|Default|GetSlowMoRecoverStart))
  (bind _slowmorecoverdur (Variables|Default|GetSlowMoRecoverDur))
  (bind _returnvalue_2 (- _returnvalue _slowmorecoverstart))
  (bind _returnvalue_3 (/ _returnvalue_2 _slowmorecoverdur))
  (bind _returnvalue_4 (Math|Float|Clamp(Float) _returnvalue_3))
  (if (Variables|Default|GetbSlowMoRecovering)
    (Variables|Default|SetCustomTimeDilation (Math|Float|Lerp (Variables|Default|GetSlowMoRecoverFrom) 1.0 _returnvalue_4))
    (if (>= _returnvalue_4 (Math|Float|MakeLiteralFloat 1.0))
      (Variables|Default|SetbSlowMoRecovering false)
      (Development|PrintString "[SlowMo] recovered" false true "(R=0.000000,G=0.660000,B=1.000000,A=1.000000)" 0.0))))

(fn TakeCombatHit
  (params (Damage :type Float%20%28double-precision%29) (PoiseDamage :type Float%20%28double-precision%29) (bForceBreak :type Boolean) (Hit :type Hit%20Result%20Structure))
  (return false))